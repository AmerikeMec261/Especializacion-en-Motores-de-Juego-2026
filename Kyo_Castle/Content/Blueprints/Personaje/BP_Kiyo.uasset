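; BP_Kiyo is the sprite-based player character Kiyo, at an early stage with movement not yet working.
; BeginPlay casts the player controller to BP_Controlador and adds the IMC_Kiyo Enhanced Input mapping context.
; A custom updaterotacion event flips the sprite according to horizontal velocity, but its only call is unwired.
; The IA_caminar walk action only prints a debug message, and the movement and offset nodes never run.
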(event Custom|update%20rotacion
  (bind _sprite (Variables|Default|GetSprite))
  (Math|Float|CompareFloat (.x (Variables|/Script/Engine.MovementComponent|GetVelocity (Variables|Character|GetCharacterMovement))) 0.0
    (:>
      (Transformation|SetRelativeRotation _sprite "0.000000,180.000000,0.000000" false false))
    (:<
      (Transformation|SetRelativeRotation _sprite "0, 0, 0" false false))))

(event Input|EnhancedActionEvents|EnhancedInputActionIA_caminar
  (params (ActionValue :type Float%20%28double-precision%29) (ElapsedSeconds :type Float%20%28double-precision%29) (TriggeredSeconds :type Float%20%28double-precision%29) (InputAction :type Input%20Action%20Object%20Reference :default "/Game/Blueprints/Personaje/IA_caminar.IA_caminar"))
  (:Started
    (Development|PrintString "Hello")))

(event EventBeginPlay
  (bind _asbp_controlador (Utilities|Casting|CastToBP_Controlador (Game|GetPlayerController 0)))
  (Utilities|IsValid (PlayerController|LocalPlayerSubsystems|GetEnhancedInputLocalPlayerSubsystem _asbp_controlador)
    (:Is%20Valid
      (Input|AddMappingContext (PlayerController|LocalPlayerSubsystems|GetEnhancedInputLocalPlayerSubsystem _asbp_controlador) "/Game/Blueprints/Personaje/IMC_Kiyo.IMC_Kiyo" 0 "(bIgnoreAllPressedKeysUntilRelease=True,bForceImmediately=False,bNotifyUserSettings=False)"))))

(event EventTick
  (params (DeltaSeconds :type Float%20%28single-precision%29)))

(fn ConstructionScript)