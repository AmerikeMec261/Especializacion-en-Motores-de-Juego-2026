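; BP_Michilago is a moving hazard that brings up the death screen when something overlaps it.
; Tick moves it along world X by Velocidad times DIRECCION, scaled by delta time.
; Overlaps on the Spherer and SphereD spheres set DIRECCION to negative or positive, reversing its travel.
; Any overlap on its Box waits briefly, then adds the PantallaMuerte widget to the viewport and pauses the game, without checking which actor entered.
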(event OnComponentBeginOverlap(Box)
  (params (OverlappedComponent :type Primitive%20Component%20Object%20Reference) (OtherActor :type Actor%20Object%20Reference) (OtherComp :type Primitive%20Component%20Object%20Reference) (OtherBodyIndex :type Integer) (bFromSweep :type Boolean) (SweepResult :type Hit%20Result%20Structure%20%28by%20ref%29))
  (Utilities|FlowControl|Delay 0.2)
  (bind _returnvalue (UserInterface|CreateWidget "/Game/Blueprints/PantallaMuerte.PantallaMuerte_C" (Game|GetPlayerController 0)))
  (UserInterface|Viewport|AddtoViewport _returnvalue 0)
  (Game|SetGamePaused true))

(event OnComponentBeginOverlap(SphereD)
  (params (OverlappedComponent :type Primitive%20Component%20Object%20Reference) (OtherActor :type Actor%20Object%20Reference) (OtherComp :type Primitive%20Component%20Object%20Reference) (OtherBodyIndex :type Integer) (bFromSweep :type Boolean) (SweepResult :type Hit%20Result%20Structure%20%28by%20ref%29))
  (Variables|Default|SetDIRECCION 1.0))

(event OnComponentBeginOverlap(Spherer)
  (params (OverlappedComponent :type Primitive%20Component%20Object%20Reference) (OtherActor :type Actor%20Object%20Reference) (OtherComp :type Primitive%20Component%20Object%20Reference) (OtherBodyIndex :type Integer) (bFromSweep :type Boolean) (SweepResult :type Hit%20Result%20Structure%20%28by%20ref%29))
  (Variables|Default|SetDIRECCION -1.0))

(event EventBeginPlay)

(event EventTick
  (params (DeltaSeconds :type Float%20%28single-precision%29))
  (bind _returnvalue (Transformation|GetActorLocation))
  (Transformation|SetActorLocation (Math|Vector|MakeVector (+ (* DeltaSeconds (Variables|Default|Getvelocidad) (Variables|Default|GetDIRECCION)) (.x _returnvalue)) (.y _returnvalue) (.z _returnvalue)) false false))

(fn ConstructionScript)